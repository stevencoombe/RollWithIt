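; Flame ball hazard that cycles on and off and drains the RBT player character's battery while it is inside the box.
; After a startup wait, a Tick-driven Active gate and latent Delays toggle the particle effect and box collision at the configurable Delay interval.
; Overlap events set a flag for RBT, and a one-second Delay on Tick paces the BatteryDrain subtraction from BatteryPower.
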(event OnComponentBeginOverlap(Box)
  (params (OverlappedComponent :type Primitive%20Component%20Object%20Reference) (OtherActor :type Actor%20Object%20Reference) (OtherComp :type Primitive%20Component%20Object%20Reference) (OtherBodyIndex :type Integer) (bFromSweep :type Boolean) (SweepResult :type Hit%20Result%20Structure%20%28by%20ref%29))
  (if (== OtherActor (Variables|Default|GetRBT))
    (Variables|Default|SetOverlapped true)))

(event OnComponentEndOverlap(Box)
  (params (OverlappedComponent :type Primitive%20Component%20Object%20Reference) (OtherActor :type Actor%20Object%20Reference) (OtherComp :type Primitive%20Component%20Object%20Reference) (OtherBodyIndex :type Integer))
  (if (== OtherActor (Variables|Default|GetRBT))
    (Variables|Default|SetOverlapped false)))

(event EventTick
  (params (DeltaSeconds :type Float%20%28single-precision%29))
  (bind _rbt (Variables|Default|GetRBT))
  (Utilities|FlowControl|Sequence
    (:then_0
      (if (Variables|Default|GetActive)
        (Variables|Default|SetActive false)
        (Utilities|FlowControl|Delay (Variables|Default|GetDelay))
        (Components|Activation|Deactivate (Variables|Default|GetP_FlameBall))
        (Collision|SetCollisionEnabled (Variables|Default|GetBox) "NoCollision")
        (Utilities|FlowControl|Delay (Variables|Default|GetDelay))
        (Components|Activation|Activate (Variables|Default|GetP_FlameBall) false)
        (Collision|SetCollisionEnabled (Variables|Default|GetBox) "QueryAndPhysics")
        (Variables|Default|SetActive true)))
    (:then_1
      (Utilities|FlowControl|Delay 1.0)
      (if (Variables|Default|GetOverlapped)
        (Variables|/Game/Blueprint/RBT_BP.RBT_BP_C|SetBatteryPower _rbt (- (Variables|/Game/Blueprint/RBT_BP.RBT_BP_C|GetBatteryPower _rbt) (Variables|Default|GetBatteryDrain)))))))

(event EventBeginPlay
  (Utilities|FlowControl|Delay 0.2)
  (Components|Activation|Deactivate (Variables|Default|GetP_FlameBall))
  (Collision|SetCollisionEnabled (Variables|Default|GetBox) "NoCollision")
  (bind _asrbt_bp (Utilities|Casting|CastToRBT_BP (Game|GetPlayerCharacter 0)))
  (Variables|Default|SetRBT _asrbt_bp)
  (Utilities|FlowControl|Delay (Variables|Default|GetDelay))
  (Components|Activation|Activate (Variables|Default|GetP_FlameBall) false)
  (Collision|SetCollisionEnabled (Variables|Default|GetBox) "QueryAndPhysics")
  (Variables|Default|SetActive true))

(fn ConstructionScript)