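; MainGameMode is a game mode that tracks the cog and circuit collection win condition for the RBT robot player.
; On begin play it sets RBT_BP as the default pawn class, then caches the player character after a short delay.
; ItemCheck compares collected counts to targets, then clears widgets, tops up the robot's battery, shows the Win widget and opens the YouWinMap level after a delay.
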(event Custom|ItemCheck
  (if (and (>= (Variables|Default|GetCogsCollected) (Variables|Default|GetCogs)) (>= (Variables|Default|GetCircuitsCollected) (Variables|Default|GetCircuits)))
    (Viewport|RemoveAllWidgets)
    (Variables|/Game/Blueprint/RBT_BP.RBT_BP_C|SetBatteryPower (Variables|Default|GetRBT) 1e+05)
    (bind _returnvalue (UserInterface|CreateWidget "/Game/UI/Win.Win_C"))
    (UserInterface|Viewport|AddtoViewport _returnvalue 0)
    (Utilities|FlowControl|Delay 3.0)
    (Game|OpenLevel(byName) "YouWinMap")))

(event EventBeginPlay
  (Variables|Default|SetDefaultPawnClass "/Game/Blueprint/RBT_BP.RBT_BP_C")
  (Utilities|FlowControl|Delay 0.2)
  (bind _asrbt_bp (Utilities|Casting|CastToRBT_BP (Game|GetPlayerCharacter 0)))
  (Variables|Default|SetRBT _asrbt_bp))

(fn ConstructionScript)