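; Crane Blueprint that drives a claw's repeating up-and-down motion through an InterpToMovement component.
; When movement begins a wait, a Delayed flag guards a timed sequence that toggles PauseOnImpact and deactivates the component after stop and retract delays.
; Deactivation waits a start delay, then reactivates the component, which restarts movement on activation to loop the cycle.
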(event OnComponentDeactivated(InterpToMovement)
  (params (Component :type Actor%20Component%20Object%20Reference))
  (Utilities|FlowControl|Delay (Variables|Default|GetClawStartDelay))
  (Components|Activation|Activate (Variables|Default|GetInterpToMovement) true))

(event OnComponentActivated(InterpToMovement)
  (params (Component :type Actor%20Component%20Object%20Reference) (bReset :type Boolean))
  (Class|InterptoMovementComponent|RestartMovement (Variables|Default|GetInterpToMovement) 1.0))

(event OnWaitBeginDelegate(InterpToMovement)
  (params (ImpactResult :type Hit%20Result%20Structure%20%28by%20ref%29) (Time :type Float%20%28single-precision%29))
  (bind _interptomovement (Variables|Default|GetInterpToMovement))
  (if (not (Variables|Default|GetDelayed))
    (Utilities|FlowControl|Delay (Variables|Default|GetClawStopTimer))
    (Variables|Default|SetDelayed true)
    (Variables|/Script/Engine.InterpToMovementComponent|SetbPauseOnImpact (Variables|Default|GetInterpToMovement) false)
    (Utilities|FlowControl|Delay (Variables|Default|GetClawRetractTimer))
    (Variables|Default|SetDelayed false)
    (Variables|/Script/Engine.InterpToMovementComponent|SetbPauseOnImpact _interptomovement true)
    (Components|Activation|Deactivate _interptomovement)))

(fn ConstructionScript)