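; SplatOne_BP is a hazard that drains the RBT player character's battery while it overlaps the actor.
; BeginPlay caches the player as RBT after a short delay, and overlap begin and end events toggle an Overlapped flag.
; While flagged, Tick runs a Delay of InvincibilityTimer that paces each BatteryDrain subtraction from BatteryPower.
; A pending drain still lands after the overlap ends.
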(event EventBeginPlay
  (Utilities|FlowControl|Delay 0.2)
  (bind _asrbt_bp (Utilities|Casting|CastToRBT_BP (Game|GetPlayerCharacter 0)))
  (Variables|Default|SetRBT _asrbt_bp))

(event Collision|EventActorBeginOverlap
  (params (OtherActor :type Actor%20Object%20Reference))
  (if (== OtherActor (Variables|Default|GetRBT))
    (Variables|Default|SetOverlapped true)))

(event EventTick
  (params (DeltaSeconds :type Float%20%28single-precision%29))
  (bind _rbt (Variables|Default|GetRBT))
  (if (Variables|Default|GetOverlapped)
    (Utilities|FlowControl|Delay (Variables|Default|GetInvincibilityTimer))
    (Variables|/Game/Blueprint/RBT_BP.RBT_BP_C|SetBatteryPower _rbt (- (Variables|/Game/Blueprint/RBT_BP.RBT_BP_C|GetBatteryPower _rbt) (Variables|Default|GetBatteryDrain)))))

(event Collision|EventActorEndOverlap
  (params (OtherActor :type Actor%20Object%20Reference))
  (if (== OtherActor (Variables|Default|GetRBT))
    (Variables|Default|SetOverlapped false)))

(fn ConstructionScript)