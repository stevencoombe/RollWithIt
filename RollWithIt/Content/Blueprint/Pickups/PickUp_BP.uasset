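; PickUp_BP is a collectible pickup that counts as a cog or circuit when an RBT_BP actor overlaps it.
; On overlap it disables collision, increments CogsCollected for a "Cog" tag or CircuitsCollected otherwise, calls ItemCheck on MainGameMode, then destroys itself.
; MainGameMode is cached shortly after BeginPlay.
; Tick spins the actor by a fixed per-frame rotation and plays a Bob timeline that offsets its location.
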(event OnComponentBeginOverlap(CollisionComp)
  (params (OverlappedComponent :type Primitive%20Component%20Object%20Reference) (OtherActor :type Actor%20Object%20Reference) (OtherComp :type Primitive%20Component%20Object%20Reference) (OtherBodyIndex :type Integer) (bFromSweep :type Boolean) (SweepResult :type Hit%20Result%20Structure%20%28by%20ref%29))
  (Utilities|Casting|CastToRBT_BP OtherActor)
  (Collision|SetCollisionEnabled (Variables|Default|GetCollisionComp) "NoCollision")
  (Utilities|PickupCheck
    (:%20%20
      (Default|ItemCheck (Variables|Default|GetGameMode))
      (Actor|DestroyActor))))

(event EventTick
  (params (DeltaSeconds :type Float%20%28single-precision%29))
  ;[1 1 1] Animation
  (Transformation|AddActorLocalRotation "0,2.000000, 0" false false)
  (bind _newtrack_0 (Timeline|Bob Play)
    (:Update
      (Transformation|AddActorLocalOffset _newtrack_0 false false))))

(event EventBeginPlay
  (Utilities|FlowControl|Delay 0.2)
  (bind _asmain_game_mode (Utilities|Casting|CastToMainGameMode (Game|GetGameMode)))
  (Variables|Default|SetGameMode _asmain_game_mode))

(fn ConstructionScript)