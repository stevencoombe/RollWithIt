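; BatteryPickup_BP is a pickup that adds BatteryAmount to the BatteryPower of the RBT_BP actor that overlaps it.
; Its Sphere overlap disables collision, adds the charge, plays a 2D pickup sound and destroys the pickup.
; Tick animates it with a fixed per-frame yaw spin, not scaled by delta time, and keeps playing a timeline whose track applies an unswept local offset.
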(event OnComponentBeginOverlap(Sphere)
  (params (OverlappedComponent :type Primitive%20Component%20Object%20Reference) (OtherActor :type Actor%20Object%20Reference) (OtherComp :type Primitive%20Component%20Object%20Reference) (OtherBodyIndex :type Integer) (bFromSweep :type Boolean) (SweepResult :type Hit%20Result%20Structure%20%28by%20ref%29))
  (bind _asrbt_bp (Utilities|Casting|CastToRBT_BP OtherActor))
  (Collision|SetCollisionEnabled (Variables|Default|GetSphere) "NoCollision")
  (Variables|/Game/Blueprint/RBT_BP.RBT_BP_C|SetBatteryPower _asrbt_bp (+ (Variables|/Game/Blueprint/RBT_BP.RBT_BP_C|GetBatteryPower _asrbt_bp) (Variables|Default|GetBatteryAmount)))
  (Audio|PlaySound2D "/Game/SFX/PickUp_Cue.PickUp_Cue" 1.0 1.0 0.0 0 0)
  (Actor|DestroyActor))

(event EventTick
  (params (DeltaSeconds :type Float%20%28single-precision%29))
  ;[1 1 1] Animation
  (Transformation|AddActorLocalRotation "0,2.000000, 0" false false)
  (bind _newtrack_0 (Timeline|Timeline_0 Play)
    (:Update
      (Transformation|AddActorLocalOffset _newtrack_0 false false))))

(fn ConstructionScript)